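; Weapon pickup Blueprint that equips the collected weapon on the player, extending a parent pickup's GiveItem event.
; After the parent logic, it writes its ItemType into a fixed inventory slot on the player controller.
; It then cycles the character's AttachNextWeapon, at most once per equipped item, stopping when the call returns that slot's number so the new weapon ends up in hand.
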(event EventBeginPlay
  (|CallParentFunction) ; This node is disabled and will not be called.\nDrag off pins to build functionality.
)

(event Collision|EventActorBeginOverlap
  (params (OtherActor :type Actor%20Object%20Reference)))

(event EventTick
  (params (DeltaSeconds :type Float%20%28single-precision%29)))

(event EventGiveItem
  (bind _mycharacter (CallFunction|GetPlayerCharacterBP))
  (|CallParentFunction)
  (CallFunction|SetSlottedItem (CallFunction|GetPlayerControllerBP) (Utilities|Struct|Make "Weapon" 2) (.ItemType (Variables|Default|GetItemType))) ; This will update the item inventory slot with\nwhich ever potion was just picked up.\n\n(This is optional)
  (Utilities|Array|ForEachLoopwithBreak (Variables|Default|GetEquippedRPGItems _mycharacter) :!label _label
    (:LoopBody
      (bind _weaponindex (CallFunction|AttachNextWeapon _mycharacter))
      (if (== _weaponindex 2)
        (goto _label Break)))))

(fn ConstructionScript
  (|CallParentFunction))